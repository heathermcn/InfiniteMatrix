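; ringAttack is a moving ring projectile that destroys chickens to earn the player score.
; It caches the player pawn on BeginPlay, then each Tick sweeps along world X by RingSpeed scaled by delta time, plus the player's unscaled Increment.
; Its TriggerZone overlap increases the player's score and destroys both actors on hitting a Chicken, or destroys only the ring on hitting a BP_Tunnel.
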(event OnComponentBeginOverlap(TriggerZone)
  (params (OverlappedComponent :type Primitive%20Component%20Object%20Reference) (OtherActor :type Actor%20Object%20Reference) (OtherComp :type Primitive%20Component%20Object%20Reference) (OtherBodyIndex :type Integer) (bFromSweep :type Boolean) (SweepResult :type Hit%20Result%20Structure%20%28by%20ref%29))
  (bind _aschicken (Utilities|Casting|CastToChicken OtherActor)
    (:then
      (Default|IncreaseScore (stale EventBeginPlay _asbp_player))
      (Actor|DestroyActor _aschicken)
      (Actor|DestroyActor))
    (:CastFailed
      (Utilities|Casting|CastToBP_Tunnel OtherActor)
      (Actor|DestroyActor))))

(event EventBeginPlay
  (bind _asbp_player (Utilities|Casting|CastToBP_Player (Game|Player|GetPlayerPawn 0))))

(event Collision|EventActorBeginOverlap
  (params (OtherActor :type Actor%20Object%20Reference)))

(event EventTick
  (params (DeltaSeconds :type Float%20%28single-precision%29))
  (Transformation|AddActorWorldOffset (Math|Vector|MakeVector (+ (* DeltaSeconds (Variables|Default|GetRingSpeed)) (Variables|/Game/InfiniteMatrix/Blueprints/BP_Player.BP_Player_C|GetIncrement (stale EventBeginPlay _asbp_player))) 0.0 0.0) true))

(fn ConstructionScript)